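; Maintenance robot pawn that follows the first-person player using AI movement.
; On BeginPlay it runs AI MoveTo toward the player character, repeating five seconds after each success, with no retry on failure.
; Tick stores its velocity and fires event dispatchers for speed and moving or stationary state.
; PatrolWaypoints is an empty stub.
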(event `self.ReceiveBeginPlay`
  (`self.Move to player`))

(event `Move to player`
  (bind _asbp_first_person_character (cast `/Game/FirstPerson/Blueprints/BP_FirstPersonCharacter` (`GameplayStatics.GetPlayerCharacter` 0)))
  (bind _output_get (set `self.Player REF` _asbp_first_person_character))
  (`|AIMoveTo` self (`self.playerPOS`) _output_get
    (:`OnSuccess`
      (`KismetSystemLibrary.Delay` 5.0)
      (`self.Move to player`))))

(event `Get Player Position`
  (set `self.playerPOS` (`self.K2_GetActorLocation` (`self.Player REF`))))

(event `self.ReceiveTick`
  (params (DeltaSeconds :type "Float (single-precision)"))
  (set `self.Speed` (`self.GetVelocity`))
  (`self.Speed_DP`)
  (bind _output_get (set `self.Not_moving` (`KismetMathLibrary.Vector_IsZero` (`self.Speed`))))
  (if _output_get
    (`self.Not_Moving_DP`)
    (else
      (`self.Moving`))))

(fn `PatrolWaypoints`)

(fn `UserConstructionScript`)