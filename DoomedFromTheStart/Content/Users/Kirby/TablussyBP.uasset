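; Handheld tablet Blueprint that the first-person player opens and closes, with on-screen function buttons that can be locked or unlocked.
; Opening and closing animates the tablet between reference transforms, toggles the render-target camera capture and swaps input with the character, using paired DoOnce gates; Q closes it.
; UnlockFunction recolours Tablet_UI button images for Scan Log, Reboot and Code Enter, or resets all three; Rotate is empty.
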(event `self.ReceiveBeginPlay`
  (`KismetSystemLibrary.Delay` 0.5)
  (bind _asbp_first_person_character (cast `/Game/FirstPerson/Blueprints/BP_FirstPersonCharacter` (`GameplayStatics.GetPlayerCharacter` 0)))
  (bind _output_get (set `self.As BP First Person Character` _asbp_first_person_character))
  (set `self.Tablet RTBP` (`/Game/FirstPerson/Blueprints/BP_FirstPersonCharacter.TabletRTBP` _output_get))
  (bind _astablet_ui (cast `/Game/Users/Kirby/Tablet_UI` (`WidgetComponent.GetWidget` (`/Game/Users/Kirby/Tablet_RT_BP.Widget` (`self.Tablet RTBP`)))))
  (set `self.As Tablet UI` _astablet_ui))

(event `OpenScreen`
  (bind _returnvalue (`GameplayStatics.GetPlayerController` 0))
  (bind _returnvalue_2 (`GameplayStatics.GetPlayerController` 0))
  (bind (_returnvalue_location _returnvalue_rotation) (`KismetMathLibrary.BreakTransform` (`SceneComponent.GetRelativeTransform` (`self.TabletCloseRef`))))
  (bind (_returnvalue_location_2 _returnvalue_rotation_2) (`KismetMathLibrary.BreakTransform` (`SceneComponent.GetRelativeTransform` (`self.TabletOpenRef`))))
  (`/Engine/EditorBlueprintResources/StandardMacros.DoOnce` false :!label _label
    (:`Completed`
      (set `SceneCaptureComponent.bCaptureEveryFrame` true (`/Game/Users/Kirby/Tablet_RT_BP.Camera` (`self.Tablet RTBP`)))
      (`SceneComponent.SetHiddenInGame` (`self.Tablet`) false false)
      (`KismetSystemLibrary.MoveComponentTo` (`self.Tablet`) _returnvalue_location_2 _returnvalue_rotation_2 true true 1.0)
      (set `self.Open` true)
      (`self.DisableInput` (`self.As BP First Person Character`) _returnvalue_2)
      (`self.EnableInput` _returnvalue_2)
      (`KismetSystemLibrary.Delay` 0.2)
      (goto _label_2 :!via `Reset`))))

(event `CLoseScreen`
  (bind _returnvalue (`GameplayStatics.GetPlayerController` 0))
  (bind (_returnvalue_location _returnvalue_rotation) (`KismetMathLibrary.BreakTransform` (`SceneComponent.GetRelativeTransform` (`self.TabletCloseRef`))))
  (`/Engine/EditorBlueprintResources/StandardMacros.DoOnce` true :!label _label_2
    (:`Completed`
      (`KismetSystemLibrary.MoveComponentTo` (`self.Tablet`) _returnvalue_location _returnvalue_rotation true true 1.0)
      (`SceneComponent.SetHiddenInGame` (`self.Tablet`) true false)
      (set `SceneCaptureComponent.bCaptureEveryFrame` false (`/Game/Users/Kirby/Tablet_RT_BP.Camera` (`self.Tablet RTBP`)))
      (set `self.Open` false)
      (`self.DisableInput` _returnvalue)
      (`self.EnableInput` (`self.As BP First Person Character`) _returnvalue)
      (`KismetSystemLibrary.Delay` 0.2)
      (goto _label :!via `Reset`))))

(event `Key|Q`
  (params (Key :type "Key Structure"))
  (:`Pressed`
    (if (`self.Open`)
      (`self.CLoseScreen`))))

(event `UnlockFunction`
  (params (`Function To Unlock` :type "/Game/Users/Charlie/CoolFolder/InteractAction Enum" :default "NewEnumerator4"))
  ; Check Which Button to Unlock
  (switch `/Game/Users/Charlie/CoolFolder/InteractAction` `Function To Unlock`
    (:`NewEnumerator4`
      (`self.LockFunctions`))
    (:`NewEnumerator0`
      (`self.Scan Log`))
    (:`NewEnumerator1`
      (`self.Reboot`))
    (:`NewEnumerator2`
      (`self.Code Enter`))
    (:`NewEnumerator3`
      (`self.Rotate`))))

(event `Scan Log`
  ;[0.04676 0.15 0.06203 0.5] Unlock Buttons
  (`Image.SetColorAndOpacity` (`/Game/Users/Kirby/Tablet_UI.Image_17` (`self.As Tablet UI`)) (struct :`R` 0.421875 :`B` 0.355181 :`A` 1.0)))

(event `Reboot`
  ;[0.04676 0.15 0.06203 0.5] Unlock Buttons
  (`Image.SetColorAndOpacity` (`/Game/Users/Kirby/Tablet_UI.Image_18` (`self.As Tablet UI`)) (struct :`R` 0.421875 :`B` 0.355181 :`A` 1.0)))

(event `Code Enter`
  ;[0.04676 0.15 0.06203 0.5] Unlock Buttons
  (`Image.SetColorAndOpacity` (`/Game/Users/Kirby/Tablet_UI.Image_19` (`self.As Tablet UI`)) (struct :`R` 0.421875 :`B` 0.355181 :`A` 1.0)))

(event `Rotate`
  ;[0.04676 0.15 0.06203 0.5] Unlock Buttons
)

(event `LockFunctions`
  (bind _as_tablet_ui (`self.As Tablet UI`))
  ;[0.15 0 0 0.5] Lock Buttons
  (`|ExecutionSequence`
    (:`then_0`
      (`Image.SetColorAndOpacity` (`/Game/Users/Kirby/Tablet_UI.Image_17` _as_tablet_ui) (struct :`R` 0.076185 :`G` 1.0 :`B` 0.082283 :`A` 1.0)))
    (:`then_1`
      (`Image.SetColorAndOpacity` (`/Game/Users/Kirby/Tablet_UI.Image_18` _as_tablet_ui) (struct :`R` 0.076185 :`G` 1.0 :`B` 0.082283 :`A` 1.0)))
    (:`then_2`
      (`Image.SetColorAndOpacity` (`/Game/Users/Kirby/Tablet_UI.Image_19` _as_tablet_ui) (struct :`R` 0.076185 :`G` 1.0 :`B` 0.082283 :`A` 1.0)))))

(fn `UserConstructionScript`)