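; Maintenance robot Blueprint that loses health while its Room is not mostly lit and dies when health runs out.
; On BeginPlay it binds to the Room's robot trigger, which starts or stops a looping one-second damage timer according to the lighting.
; Each tick of that timer removes one health and prints a debug value.
; A Rebooted event refills health but leaves the Dead flag untouched.
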(event `self.ReceiveBeginPlay`
  (add `/Game/Users/WilliamG/Space_n_light/Lumninance_Detector.Trigger Robots` (`self.Room`) (delegate `CheckLuminance`)))

(event `CheckLuminance`
  (if (`self.Dead`)
    _
    (elif (`/Game/Users/WilliamG/Space_n_light/Lumninance_Detector.Room Is Mostly Lit` (`self.Room`))
      (`self.StopTimer`)
      (else
        (`self.StartTimer`)))))

(event `Rebooted`
  (set `self.Health` 720))

(event `StartTimer`
  (bind _returnvalue (`KismetSystemLibrary.K2_SetTimerDelegate` (delegate `TakeDamage`) 1.0 true)))

(event `StopTimer`
  (`KismetSystemLibrary.K2_ClearAndInvalidateTimerHandle` (stale `StartTimer` _returnvalue)))

(event `TakeDamage`
  (bind _returnvalue (- (`self.Health`) 1))
  (bind _output_get (set `self.Health` _returnvalue))
  (`|ExecutionSequence`
    (:`then_0`
      (if (< _output_get 1)
        (`self.StopTimer`)
        (`self.RobotDied`)))
    (:`then_1`
      (`KismetSystemLibrary.PrintString` (`KismetStringLibrary.Conv_IntToString` _returnvalue)))))

(event `RobotDied`
  (set `self.Dead` true))

(fn `UserConstructionScript`)