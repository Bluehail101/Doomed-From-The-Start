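; Daisy enemy AI that patrols BP_Daisy_Waypoint actors, chases the player on sight and disables their input when caught.
; Patrol loops through waypoints with AIMoveTo, and PawnSensing starts the faster chase when attacking is allowed.
; Delay-throttled Tick checks trace from the player, dropping the chase after sustained blocked sight.
; SUNDETECTOR light state drives spotlight color and, through DoOnce gates, pauses movement and toggles attack ability.
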(event `PatrolWaypoints`
  (bind _currentindex (`self.CurrentIndex`))
  (bind _returnvalue (`KismetStringLibrary.Concat_StrStr` "Patrol: " (`KismetStringLibrary.Conv_IntToString` _currentindex)))
  (if (`self.Is Patrolling`)
    (`SkeletalMeshComponent.PlayAnimation` (`self.Mesh`) "/Game/Characters/Mannequins/Anims/Unarmed/Walk/MF_Unarmed_Walk_Fwd.MF_Unarmed_Walk_Fwd" true)
    (`|AIMoveTo` self (0.0 0.0 0.0) (`|GetArrayItem` (`self.waypoints`) (`self.CurrentIndex`))
      (:`OnSuccess`
        (`/Engine/EditorBlueprintResources/StandardMacros.IncrementInt` (`self.CurrentIndex`)
          (:`  `
            (if (>= _currentindex (`KismetArrayLibrary.Array_Length` (`self.waypoints`)))
              (set `self.CurrentIndex` 0))
            (bind _output_get (set `self.TestText` _returnvalue))
            (`KismetSystemLibrary.PrintString` _output_get)
            (`TextRenderComponent.K2_SetText` (`self.StateText`) (`KismetTextLibrary.Conv_StringToText` _returnvalue))
            (`SkeletalMeshComponent.PlayAnimation` (`self.Mesh`) "/Game/Characters/Mannequins/Anims/Unarmed/MM_Idle.MM_Idle" true)
            (`KismetSystemLibrary.Delay` 1.0)
            (`self.PatrolWaypoints`)))))))

(event `self.PawnSensing.OnSeePawn`
  (params (Pawn :type "Pawn Object Reference"))
  (if (`self.Can attack`)
    (if (`self.Is Chase Active`)
      _
      (elif (== Pawn (`GameplayStatics.GetPlayerPawn` 0))
        (`self.Trigger Chase`)))))

(event `self.ReceiveBeginPlay`
  (bind _outactors (`GameplayStatics.GetAllActorsOfClass` "/Game/Users/WillC/BP_Daisy_Waypoint.BP_Daisy_Waypoint_C"))
  (set `self.waypoints` _outactors)
  (`self.PatrolWaypoints`))

(event `self.ReceiveTick`
  (params (DeltaSeconds :type "Float (single-precision)"))
  (bind _sundetector (`self.SUNDETECTOR`))
  (bind _spotlight (`self.SpotLight`))
  (bind _charactermovement (`self.CharacterMovement`))
  (`|ExecutionSequence`
    (:`then_0`
      (`KismetSystemLibrary.Delay` 0.2)
      (if (`/Game/Users/WilliamG/Space_n_light/In_SunLight_Detector.Daisy Is In Light` _sundetector)
        (`|ExecutionSequence`
          (:`then_0`
            (`LightComponent.SetLightColor` _spotlight (make `LinearColor` 0.0 1.0) true))
          (:`then_1`
            (goto _label_2 :!via `Reset`))
          (:`then_2`
            (`/Engine/EditorBlueprintResources/StandardMacros.DoOnce` false :!label _label
              (:`Completed`
                (`MovementComponent.StopMovementImmediately` _charactermovement)
                (set `CharacterMovementComponent.MaxWalkSpeed` 300.0 _charactermovement)
                (`SkeletalMeshComponent.PlayAnimation` (`self.Mesh`) "/Game/Characters/Mannequins/Anims/Unarmed/MM_Idle.MM_Idle" true)
                (set `self.Can attack` false)
                (`KismetSystemLibrary.Delay` 5.0)
                (set `self.Is Patrolling` true)
                (`self.PatrolWaypoints`)))))
        (else
          (`|ExecutionSequence`
            (:`then_0`
              (`/Engine/EditorBlueprintResources/StandardMacros.DoOnce` false :!label _label_2
                (:`Completed`
                  (set `self.Is Patrolling` false)
                  (`MovementComponent.StopMovementImmediately` (`self.CharacterMovement`))
                  (`SkeletalMeshComponent.PlayAnimation` (`self.Mesh`) "/Game/Characters/Mannequins/Anims/Unarmed/MM_Idle.MM_Idle" true)
                  (`KismetSystemLibrary.Delay` 5.0)
                  (set `self.Is Patrolling` true)
                  (`self.PatrolWaypoints`)
                  (set `self.Can attack` true))))
            (:`then_1`
              (if (and (!= (`/Game/Users/WilliamG/Space_n_light/In_SunLight_Detector.Player Is In Light` _sundetector) true) (`self.Is Chase Active`))
                (`LightComponent.SetLightColor` _spotlight (make `LinearColor` 1.0) true)
                (else
                  (`LightComponent.SetLightColor` _spotlight (make `LinearColor` 1.0 1.0) true))))
            (:`then_2`
              (goto _label :!via `Reset`))))))
    (:`then_1`
      (`KismetSystemLibrary.Delay` 1.0)
      (if (`self.Is Chase Active`)
        (bind (_outhit _returnvalue) (`KismetSystemLibrary.LineTraceSingle` :`Start` (`self.K2_GetActorLocation` (`GameplayStatics.GetPlayerCharacter` 0)) :`End` (`SceneComponent.K2_GetComponentLocation` (`self.CapsuleComponent`)) :`TraceChannel` "TraceTypeQuery1" :`DrawDebugType` "ForDuration" :`TraceColor` (struct :`G` 0.409775 :`B` 1.0 :`A` 1.0) :`TraceHitColor` (struct :`R` 1.0 :`G` 0.999582 :`A` 1.0) :`DrawTime` 2.0))
        (if _returnvalue
          (bind _output_get (set `self.Time Not Visible` (+ 1.0 (`self.Time Not Visible`))))
          (if (>= _output_get 5.0)
            (`MovementComponent.StopMovementImmediately` (`self.CharacterMovement`))
            (`KismetSystemLibrary.PrintString` "LOSAT")
            (set `self.Time Not Visible` 0.0)
            (set `self.Is Chase Active` false :!label _label_3)
            (set `CharacterMovementComponent.MaxWalkSpeed` 300.0 (`self.CharacterMovement`))
            (`SkeletalMeshComponent.PlayAnimation` (`self.Mesh`) "/Game/Characters/Mannequins/Anims/Unarmed/MM_Idle.MM_Idle" true)
            (`KismetSystemLibrary.Delay` 5.0)
            (set `self.Is Patrolling` true)
            (`self.PatrolWaypoints`)
            (else
              (`KismetSystemLibrary.PrintString` (`KismetStringLibrary.Conv_DoubleToString` _output_get))))
          (else
            (set `self.Time Not Visible` 0.0)))))))

(event `Trigger Chase`
  (bind _returnvalue (`GameplayStatics.GetPlayerPawn` 0))
  (bind _mesh (`self.Mesh`))
  (bind _charactermovement (`self.CharacterMovement`))
  (set `self.Is Chase Active` true)
  (set `self.Is Patrolling` false)
  (`SkeletalMeshComponent.PlayAnimation` _mesh "/Game/Characters/Mannequins/Anims/Unarmed/MM_Idle.MM_Idle" true)
  (`MovementComponent.StopMovementImmediately` _charactermovement)
  (`KismetSystemLibrary.Delay` 1.0)
  (set `CharacterMovementComponent.MaxWalkSpeed` 600.0 _charactermovement)
  (`SkeletalMeshComponent.PlayAnimation` _mesh "/Game/Characters/Mannequins/Anims/Unarmed/Jog/MF_Unarmed_Jog_Fwd.MF_Unarmed_Jog_Fwd" true)
  (`|AIMoveTo` self (0.0 0.0 0.0) _returnvalue
    (:`then`
      (`KismetSystemLibrary.PrintString` "I see you!"))
    (:`OnSuccess`
      (`SkeletalMeshComponent.PlayAnimation` _mesh "/Game/Characters/Mannequins/Anims/Unarmed/MM_Idle.MM_Idle" true)
      (`self.DisableInput` _returnvalue (`GameplayStatics.GetPlayerController` 0))
      (`KismetSystemLibrary.PrintString` "I got you"))
    (:`OnFail`
      (goto _label_3))))

(fn `UserConstructionScript`)