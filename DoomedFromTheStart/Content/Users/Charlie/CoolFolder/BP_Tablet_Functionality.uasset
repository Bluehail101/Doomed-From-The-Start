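; BP_Tablet_Functionality handles the player toggling a tablet open and closed with the F key.
; The key press is ignored while PreventTabletUse is set; otherwise ToggleTablet flips the Using flag and calls OpenTablet or CloseTablet.
; Opening disables input on the pawn controlled by player 0 and closing restores it; no tablet display logic is present.
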(event `Key|F` :consume false
  (params (Key :type "Key Structure"))
  (:`Pressed`
    (if (not (`self.PreventTabletUse`))
      (`self.ToggleTablet`))))

(event `ToggleTablet`
  (if (`self.Using`)
    (set `self.Using` false)
    (`self.CloseTablet`)
    (else
      (set `self.Using` true)
      (`self.OpenTablet`))))

(event `OpenTablet`
  (bind _returnvalue (`GameplayStatics.GetPlayerController` 0))
  (`self.DisableInput` (`Controller.K2_GetPawn` _returnvalue) _returnvalue))

(event `CloseTablet`
  (bind _returnvalue (`GameplayStatics.GetPlayerController` 0))
  (`self.EnableInput` (`Controller.K2_GetPawn` _returnvalue) _returnvalue))

(fn `UserConstructionScript`)