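; BP_Interactable is a trigger-based interactable that shows a text prompt while the player overlaps it and responds to F.
; InteractType selects Tap, Pickup or Hold, which broadcast the Interacted dispatcher for other logic to bind.
; Pickup also calls PickedUp on PickupObject and disables itself.
; Hold alternates via FlipFlop between disabling pawn input with Interacted and re-enabling it with Uninteracted, toggling per press rather than tracking key release.
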(event `Set On or Off`
  (params (On :type Boolean))
  ;[1 1 1 0.5] Toggle if trigger is on or not
  (bind _output_get (set `self.On` On))
  (set `PrimitiveComponent.bGenerateOverlapEvents` _output_get (`self.Trigger`)))

(event `Tap`
  ; Tap Type
  (`self.Call Interact Dispatcher`))

(event `Pickup`
  ; Pickup Type
  (`self.Call Interact Dispatcher`)
  (`/Game/Users/Charlie/CoolFolder/BP_Pickup.Picked Up` (`self.PickupObject`))
  (`self.Set On or Off` false)
  (`self.InteractTextVisibility` false))

(event `self.ReceiveBeginPlay`
  ;[1 1 1 0.5] Start
  (`self.SetInteractText`)
  (`self.Set On or Off` (`self.On`)))

(event `Hold`
  (bind _returnvalue (`GameplayStatics.GetPlayerController` 0))
  (bind _returnvalue_2 (`Controller.K2_GetPawn` _returnvalue))
  ; Hold Type
  (`/Engine/EditorBlueprintResources/StandardMacros.FlipFlop`
    (:`A`
      (`self.Call Interact Dispatcher`)
      (`self.DisableInput` _returnvalue_2 _returnvalue))
    (:`B`
      (`self.Call Uninteract Dispatcher`)
      (`self.EnableInput` _returnvalue_2 _returnvalue))))

(event `self.Trigger.OnComponentBeginOverlap`
  (params (OverlappedComponent :type "PrimitiveComponent Object Reference") (OtherActor :type "Actor Object Reference") (OtherComp :type "PrimitiveComponent Object Reference") (OtherBodyIndex :type Integer) (bFromSweep :type Boolean) (SweepResult :type "HitResult Structure (by ref)"))
  ;[1 1 1 0.5] Events for when player steps in and out of trigger
  (if (== OtherActor (`GameplayStatics.GetPlayerCharacter` 0))
    (set `self.InTrigger` true)
    (`SceneComponent.SetVisibility` (`self.InteractText`) true false)))

(event `self.Trigger.OnComponentEndOverlap`
  (params (OverlappedComponent :type "PrimitiveComponent Object Reference") (OtherActor :type "Actor Object Reference") (OtherComp :type "PrimitiveComponent Object Reference") (OtherBodyIndex :type Integer))
  ;[1 1 1 0.5] Events for when player steps in and out of trigger
  (if (== (`GameplayStatics.GetPlayerCharacter` 0) OtherActor)
    (set `self.InTrigger` false)
    (`SceneComponent.SetVisibility` (`self.InteractText`) false false)))

(event `Call Interact Dispatcher`
  ; Dispatchers
  (`self.Interacted`))

(event `Key|F` :consume false
  (params (Key :type "Key Structure"))
  ;[1 1 1 0.5] Player interact attempt & check interact type
  (:`Pressed`
    (if (`self.InTrigger`)
      (switch `/Game/Users/Charlie/CoolFolder/InteractType` (`self.InteractType`)
        (:`NewEnumerator0`
          (`self.Tap`))
        (:`NewEnumerator1`
          (`self.Pickup`))
        (:`NewEnumerator2`
          (`self.Hold`))))))

(event `Call Uninteract Dispatcher`
  ; Dispatchers
  (`self.Uninteracted`))

(event `SetInteractText`
  ;[1 1 1 0.5] Interact Text Events
  (`self.InteractTextVisibility` false)
  (`TextRenderComponent.K2_SetText` (`self.InteractText`) (`KismetTextLibrary.Conv_StringToText` (`self.InteractPrompt`))))

(event `InteractTextVisibility`
  (params (On :type Boolean))
  ;[1 1 1 0.5] Interact Text Events
  (`SceneComponent.SetVisibility` (`self.InteractText`) On false))

(fn `GetInteractEvent`
  (returns (NewParam :type "StateTreeDelegateDispatcher Structure"))
  (return))

(fn `UserConstructionScript`)