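; BP_TabletInteract is a trigger that changes which function is unlocked on the player's tablet while the player stands inside it.
; On BeginPlay it applies its On state to the trigger's overlap events and caches the TablussyBP actor, printing a warning if none exists.
; Player entry unlocks the configured InteractAction after a short delay, and exit passes a fixed enum value instead.
; SetOnorOff toggles the trigger.
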(event `Set On or Off`
  (params (On :type Boolean))
  ;[1 1 1 0.5] Toggle if trigger is on or not
  (bind _output_get (set `self.On` On))
  (set `PrimitiveComponent.bGenerateOverlapEvents` _output_get (`self.Trigger`)))

(event `self.ReceiveBeginPlay`
  ;[1 1 1 0.5] Start
  (`self.Set On or Off` (`self.On`))
  (bind _returnvalue (`GameplayStatics.GetActorOfClass` "/Game/Users/Kirby/TablussyBP.TablussyBP_C"))
  (`/Engine/EditorBlueprintResources/StandardMacros.IsValid` _returnvalue
    (:`Is Valid`
      (set `self.Tablet` _returnvalue))
    (:`Is Not Valid`
      (`KismetSystemLibrary.PrintString` "Tablet Not Found ):"))))

(event `self.Trigger.OnComponentBeginOverlap`
  (params (OverlappedComponent :type "PrimitiveComponent Object Reference") (OtherActor :type "Actor Object Reference") (OtherComp :type "PrimitiveComponent Object Reference") (OtherBodyIndex :type Integer) (bFromSweep :type Boolean) (SweepResult :type "HitResult Structure (by ref)"))
  ;[1 1 1 0.5] Events for when player steps in and out of trigger
  (if (== OtherActor (`GameplayStatics.GetPlayerCharacter` 0))
    (set `self.InTrigger` true)
    (`KismetSystemLibrary.Delay` 0.1)
    (`/Game/Users/Kirby/TablussyBP.UnlockFunction` (`self.Tablet`) (`self.InteractAction`))))

(event `self.Trigger.OnComponentEndOverlap`
  (params (OverlappedComponent :type "PrimitiveComponent Object Reference") (OtherActor :type "Actor Object Reference") (OtherComp :type "PrimitiveComponent Object Reference") (OtherBodyIndex :type Integer))
  ;[1 1 1 0.5] Events for when player steps in and out of trigger
  (if (== (`GameplayStatics.GetPlayerCharacter` 0) OtherActor)
    (set `self.InTrigger` false)
    (`/Game/Users/Kirby/TablussyBP.UnlockFunction` (`self.Tablet`) "NewEnumerator4")))

(fn `UserConstructionScript`)