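; Elevator actor that moves its floor when the first player's pawn enters its trigger box.
; An Elevator selector picks the Tower or Lobby timeline, each driving the floor's relative location, with a FlipFlop alternating forward and reverse trips.
; A Permission flag blocks retriggering until the timeline finishes and prints a debug label.
; The flag clears before the pawn check, so another overlapping actor can leave the elevator locked.
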(event `self.Box.OnComponentBeginOverlap`
  (params (OverlappedComponent :type "PrimitiveComponent Object Reference") (OtherActor :type "Actor Object Reference") (OtherComp :type "PrimitiveComponent Object Reference") (OtherBodyIndex :type Integer) (bFromSweep :type Boolean) (SweepResult :type "HitResult Structure (by ref)"))
  (if (`self.Permission`)
    (set `self.Permission` false)
    (if (== OtherActor (`GameplayStatics.GetPlayerPawn` 0))
      (switch `int` (`self.Elevator`)
        (:`0`
          (`/Engine/EditorBlueprintResources/StandardMacros.FlipFlop`
            (:`A`
              (bind (_direction _tower) (`Timeline|Tower` :!label _label)
                (:`Update`
                  (`SceneComponent.K2_SetRelativeLocation` (`self.Elevator_Floor`) _tower false false))
                (:`Finished`
                  (set `self.Permission` true)
                  (`KismetSystemLibrary.PrintString` "tower"))))
            (:`B`
              (goto _label :!via `Reverse`))))
        (:`1`
          (`/Engine/EditorBlueprintResources/StandardMacros.FlipFlop`
            (:`A`
              (bind (_direction_2 _lobby) (`Timeline|Lobby` :!label _label_2)
                (:`Update`
                  (`SceneComponent.K2_SetRelativeLocation` (`self.Elevator_Floor`) _lobby false false))
                (:`Finished`
                  (set `self.Permission` true)
                  (`KismetSystemLibrary.PrintString` "lobby"))))
            (:`B`
              (goto _label_2 :!via `Reverse`))))))))

(fn `UserConstructionScript`)