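; BP_ElevatorDoor is an elevator door that slides open when the player, a Daisy AI or Will enters its trigger box, and closes when they leave.
; On overlap, it compares its TOP flag with DadElevator's UP state, summoning the elevator and waiting briefly if it is on the other level.
; One MoveComponentTo node eases StaticMesh1 along Y, retargeted between open and closed offsets.
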(event `self.Box.OnComponentBeginOverlap`
  (params (OverlappedComponent :type "PrimitiveComponent Object Reference") (OtherActor :type "Actor Object Reference") (OtherComp :type "PrimitiveComponent Object Reference") (OtherBodyIndex :type Integer) (bFromSweep :type Boolean) (SweepResult :type "HitResult Structure (by ref)"))
  (bind _returnvalue (`GameplayStatics.GetObjectClass` OtherActor))
  (bind _up_ (`/Game/Users/AlexanderJ/_GENERATED/Alex/BP_Elevator.UP?` (`self.Dad_Elevator`)))
  (if (or (== _returnvalue "/Game/FirstPerson/Blueprints/BP_FirstPersonCharacter.BP_FirstPersonCharacter_C") (== _returnvalue "/Game/Users/WillC/DEPRECATED_BP_Daisy_AI_01.DEPRECATED_BP_Daisy_AI_01_C") (== _returnvalue "/Game/Users/WilliamG/Daisy_AI/Daisy_AI_Tree.Daisy_AI_Tree_C") (== _returnvalue "/Game/Users/WilliamG/Worker_Bots/MR_BP_Will.MR_BP_Will_C"))
    (if (`self.TOP`)
      (if (not _up_)
        (`/Game/Users/AlexanderJ/_GENERATED/Alex/BP_Elevator.SummonElevator` (`self.Dad_Elevator`) :!label _label)
        (`KismetSystemLibrary.Delay` 2.0))
      (elif _up_
        (goto _label)
        (else
          _)))
    (`|ExecutionSequence`
      (:`then_0`
        (goto _label_2 :!via `Return`))
      (:`then_1`
        (set `self.Target Location` 300.0)
        (`KismetSystemLibrary.MoveComponentTo` (`self.StaticMesh1`) (`KismetMathLibrary.MakeVector` 0.0 (`self.Target Location`)) (struct) true true 1.0 :!label _label_2)))))

(event `self.Box.OnComponentEndOverlap`
  (params (OverlappedComponent :type "PrimitiveComponent Object Reference") (OtherActor :type "Actor Object Reference") (OtherComp :type "PrimitiveComponent Object Reference") (OtherBodyIndex :type Integer))
  (bind _returnvalue (`GameplayStatics.GetObjectClass` OtherActor))
  (if (or (== _returnvalue "/Game/FirstPerson/Blueprints/BP_FirstPersonCharacter.BP_FirstPersonCharacter_C") (== _returnvalue "/Game/Users/WillC/DEPRECATED_BP_Daisy_AI_01.DEPRECATED_BP_Daisy_AI_01_C") (== _returnvalue "/Game/Users/WilliamG/Daisy_AI/Daisy_AI_Tree.Daisy_AI_Tree_C") (== _returnvalue "/Game/Users/WilliamG/Worker_Bots/MR_BP_Will.MR_BP_Will_C"))
    (`|ExecutionSequence`
      (:`then_0`
        (goto _label_2 :!via `Return`))
      (:`then_1`
        (set `self.Target Location` 0.0)
        (goto _label_2)))))

(fn `UserConstructionScript`)